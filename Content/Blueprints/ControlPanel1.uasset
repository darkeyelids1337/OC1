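; Keypad control panel where the player types a fixed code to set the Lvl3Exit flag on BP_Adam.
; When BP_Adam without that flag overlaps the box, a text shows for four seconds before input is enabled; leaving disables input.
; Number keys feed TextScreen, which keeps a rolling four-digit entry shown on a TextRender.
; Backspace clears the entry, and Enter checks it against the hardcoded code.
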(event OnComponentBeginOverlap(Box)
  (params (OverlappedComponent :type Primitive%20Component%20Object%20Reference) (OtherActor :type Actor%20Object%20Reference) (OtherComp :type Primitive%20Component%20Object%20Reference) (OtherBodyIndex :type Integer) (bFromSweep :type Boolean) (SweepResult :type Hit%20Result%20Structure%20%28by%20ref%29))
  (bind _textrender1 (Variables|Default|GetTextRender1))
  (bind _asbp_adam (Utilities|Casting|CastToBP_Adam OtherActor))
  (if (not (Variables|/Game/MetaHumans/1pers/BP_Adam.BP_Adam_C|Getlvl3Exit _asbp_adam))
    (Rendering|SetVisibility _textrender1 true false)
    (Utilities|FlowControl|Delay 4.0)
    (Rendering|SetVisibility _textrender1 false false)
    (Input|EnableInput (Game|GetPlayerController 0))
    (bind _asbp_adam_2 (Utilities|Casting|CastToBP_Adam OtherActor))))

(event OnComponentEndOverlap(Box)
  (params (OverlappedComponent :type Primitive%20Component%20Object%20Reference) (OtherActor :type Actor%20Object%20Reference) (OtherComp :type Primitive%20Component%20Object%20Reference) (OtherBodyIndex :type Integer))
  (Input|DisableInput (Game|GetPlayerController 0)))

(event Input|KeyboardEvents|Enter
  (params (Key :type Key%20Structure :default "None"))
  (:Pressed
    (if (Utilities|Enum|Equal(Enum) (Variables|Default|GettempCode) "6208")
      (Variables|/Game/MetaHumans/1pers/BP_Adam.BP_Adam_C|Setlvl3Exit (stale OnComponentBeginOverlap(Box) _asbp_adam_2) true))))

(event Input|KeyboardEvents|8
  (params (Key :type Key%20Structure :default "None"))
  (:Pressed
    (bind _returnvalue (CallFunction|TextScreen (Variables|Default|GettempCode) 8))
    (bind _output_get (Variables|Default|SettempCode _returnvalue))
    (Rendering|Components|TextRender|SetText (Variables|Default|GetTextRender) (Utilities|Text|ToText(String) _output_get))))

(event Input|KeyboardEvents|9
  (params (Key :type Key%20Structure :default "None"))
  (:Pressed
    (bind _returnvalue (CallFunction|TextScreen (Variables|Default|GettempCode) 9))
    (bind _output_get (Variables|Default|SettempCode _returnvalue))
    (Rendering|Components|TextRender|SetText (Variables|Default|GetTextRender) (Utilities|Text|ToText(String) _output_get))))

(event Input|KeyboardEvents|Backspace
  (params (Key :type Key%20Structure :default "None"))
  (:Pressed
    (bind _output_get (Variables|Default|SettempCode ""))
    (Rendering|Components|TextRender|SetText (Variables|Default|GetTextRender) (Utilities|Text|ToText(String) _output_get))))

(event Input|KeyboardEvents|1
  (params (Key :type Key%20Structure :default "None"))
  (:Pressed
    (bind _returnvalue (CallFunction|TextScreen (Variables|Default|GettempCode) 1))
    (bind _output_get (Variables|Default|SettempCode _returnvalue))
    (Rendering|Components|TextRender|SetText (Variables|Default|GetTextRender) (Utilities|Text|ToText(String) _output_get))))

(event Input|KeyboardEvents|0
  (params (Key :type Key%20Structure :default "None"))
  (:Pressed
    (bind _returnvalue (CallFunction|TextScreen (Variables|Default|GettempCode)))
    (bind _output_get (Variables|Default|SettempCode _returnvalue))
    (Rendering|Components|TextRender|SetText (Variables|Default|GetTextRender) (Utilities|Text|ToText(String) _output_get))))

(event Input|KeyboardEvents|2
  (params (Key :type Key%20Structure :default "None"))
  (:Pressed
    (bind _returnvalue (CallFunction|TextScreen (Variables|Default|GettempCode) 2))
    (bind _output_get (Variables|Default|SettempCode _returnvalue))
    (Rendering|Components|TextRender|SetText (Variables|Default|GetTextRender) (Utilities|Text|ToText(String) _output_get))))

(event Input|KeyboardEvents|3
  (params (Key :type Key%20Structure :default "None"))
  (:Pressed
    (bind _returnvalue (CallFunction|TextScreen (Variables|Default|GettempCode) 3))
    (bind _output_get (Variables|Default|SettempCode _returnvalue))
    (Rendering|Components|TextRender|SetText (Variables|Default|GetTextRender) (Utilities|Text|ToText(String) _output_get))))

(event Input|KeyboardEvents|4
  (params (Key :type Key%20Structure :default "None"))
  (:Pressed
    (bind _returnvalue (CallFunction|TextScreen (Variables|Default|GettempCode) 4))
    (bind _output_get (Variables|Default|SettempCode _returnvalue))
    (Rendering|Components|TextRender|SetText (Variables|Default|GetTextRender) (Utilities|Text|ToText(String) _output_get))))

(event Input|KeyboardEvents|5
  (params (Key :type Key%20Structure :default "None"))
  (:Pressed
    (bind _returnvalue (CallFunction|TextScreen (Variables|Default|GettempCode) 5))
    (bind _output_get (Variables|Default|SettempCode _returnvalue))
    (Rendering|Components|TextRender|SetText (Variables|Default|GetTextRender) (Utilities|Text|ToText(String) _output_get))))

(event Input|KeyboardEvents|6
  (params (Key :type Key%20Structure :default "None"))
  (:Pressed
    (bind _returnvalue (CallFunction|TextScreen (Variables|Default|GettempCode) 6))
    (bind _output_get (Variables|Default|SettempCode _returnvalue))
    (Rendering|Components|TextRender|SetText (Variables|Default|GetTextRender) (Utilities|Text|ToText(String) _output_get))))

(event Input|KeyboardEvents|7
  (params (Key :type Key%20Structure :default "None"))
  (:Pressed
    (bind _returnvalue (CallFunction|TextScreen (Variables|Default|GettempCode) 7))
    (bind _output_get (Variables|Default|SettempCode _returnvalue))
    (Rendering|Components|TextRender|SetText (Variables|Default|GetTextRender) (Utilities|Text|ToText(String) _output_get))))

(fn ConstructionScript)

(fn TextScreen
  (params (tempCode :type String) (PressedButton :type Integer))
  (return (Utilities|String|Append (Utilities|String|Right tempCode 3) (Utilities|String|ToString(Integer) PressedButton))))